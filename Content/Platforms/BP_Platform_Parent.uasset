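; Parent Blueprint for platforms that can shuttle back and forth and react to characters standing on or touching them.
; If CanMove is set, a self-restarting timeline lerps Platform between the StartMesh and EndMesh transforms, scaled by PlayRate.
; Overlaps add new characters to an array and pass indices to empty Activate/Deactivate hooks; this class never removes entries.
; The construction script shows the endpoint meshes in red or hides them with an invisible material.
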(event Custom|Moving%20Event
  ;[0.15 0.15 0.15 0.5] Movement
  (if (Variables|Default|GetCanMove)
    (Components|Timeline|SetPlayRate (Variables|Default|GetMoving) (/ 1.0 (Variables|Default|GetPlayRate)))
    (switch Utilities|FlowControl|Switch|SwitchonETimelineDirection (Variables|Default|GetDirection)
      (:Forward
        (bind (_direction _moving) (Timeline|Moving ReverseFromEnd)
          (:Update
            (Transformation|SetWorldTransform (Variables|Default|GetPlatform) (Math|Transform|Lerp(Transform) (Transformation|GetWorldTransform (Variables|Default|GetStartMesh)) (Transformation|GetWorldTransform (Variables|Default|GetEndMesh)) _moving) false false))
          (:Finished
            (Variables|Default|SetDirection _direction)
            (CallFunction|MovingEvent))))
      (:Backward
        (Timeline|Moving PlayFromStart)))))

(event EventBeginPlay
  (CallFunction|MovingEvent))

(event Collision|EventActorBeginOverlap
  (params (OtherActor :type Actor%20Object%20Reference))
  (bind _ascharacter (Utilities|Casting|CastToCharacter OtherActor))
  (if (not (.IsOverlapping1 (CallFunction|CheckOverlapArray _ascharacter)))
    (bind _returnvalue (Utilities|Array|Add (Variables|Default|GetOverlappin%20Actors) _ascharacter))
    (CallFunction|ActivatePlatform _returnvalue)))

(event Collision|EventActorEndOverlap
  (params (OtherActor :type Actor%20Object%20Reference))
  (bind _ascharacter (Utilities|Casting|CastToCharacter OtherActor))
  (if (.IsOverlapping1 (CallFunction|CheckOverlapArray _ascharacter))
    (CallFunction|DeactivatePlatform (.Index (CallFunction|CheckOverlapArray _ascharacter)))))

(fn ConstructionScript
  (bind _startmesh (Variables|Default|GetStartMesh))
  (if (Variables|Default|GetShowStartEndMesh)
    (Rendering|Material|SetMaterial _startmesh 0 "/Game/Platforms/Material/M_RedMesh.M_RedMesh")
    (else
      (Rendering|Material|SetMaterial _startmesh 0 "/Game/Platforms/Material/M_Invis.M_Invis"))))

(fn CheckOverlapArray
  (params (Overlap%20Actor :type Character%20Object%20Reference))
  (for (_array_element _array_index) (Variables|Default|GetOverlappin%20Actors)
    (if (== _array_element Overlap%20Actor)
      (LocalVariables|SetIsOverlapping true)
      (LocalVariables|Settemp%20Index _array_index)))
  (if (LocalVariables|GetIsOverlapping)
    (return true (LocalVariables|Gettemp%20Index))
    (else
      (return false -1))))

(fn ActivatePlatform
  (params (Index :type Integer)))

(fn DeactivatePlatform
  (params (Index :type Integer)))

(fn CheckOverlapActor
  (params (Actor :type Actor%20Object%20Reference) (Platform%20Filter :type Actor%20Class%20Reference))
  (for _array_element (Collision|GetOverlappingActors Actor Platform%20Filter :!class /Script/Engine.Actor)
    (if (Class|GameplayStatics|ObjectIsA _array_element Platform%20Filter)
      (LocalVariables|SetIsOverlapping true)))
  (return (LocalVariables|GetIsOverlapping)))