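; BP_Platform_Ice is a platform that makes characters on it slide by lowering their ground friction, acceleration and walking braking.
; ActivatePlatform applies the slippery CharacterMovement values to the overlapping actor at a given index.
; DeactivatePlatform writes back fixed normal values, rather than saved originals, and removes that actor from the array.
; The event graph is empty apart from disabled stubs, so neither function is called within this file.
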(event EventBeginPlay
  (|CallParentFunction) ; This node is disabled and will not be called.\nDrag off pins to build functionality.
)

(event Collision|EventActorBeginOverlap
  (params (OtherActor :type Actor%20Object%20Reference))
  (|CallParentFunction OtherActor) ; This node is disabled and will not be called.\nDrag off pins to build functionality.
)

(event EventTick
  (params (DeltaSeconds :type Float%20%28single-precision%29)))

(fn ConstructionScript
  (|CallParentFunction))

(fn ActivatePlatform
  (params (Index :type Integer))
  (bind _overlappin_actors (Variables|Default|GetOverlappin%20Actors))
  (bind _output (Utilities|Array|Get(acopy) _overlappin_actors Index))
  (bind _charactermovement (Variables|/Script/Engine.Character|GetCharacterMovement _output))
  (Variables|/Script/Engine.CharacterMovementComponent|SetGroundFriction _charactermovement 0.8)
  (Variables|/Script/Engine.CharacterMovementComponent|SetMaxAcceleration _charactermovement 1.5e+02)
  (Variables|/Script/Engine.CharacterMovementComponent|SetBrakingDecelerationWalking _charactermovement 2e+02))

(fn DeactivatePlatform
  (params (Index :type Integer))
  (bind _overlappin_actors (Variables|Default|GetOverlappin%20Actors))
  (bind _output (Utilities|Array|Get(acopy) _overlappin_actors Index))
  (bind _charactermovement (Variables|/Script/Engine.Character|GetCharacterMovement _output))
  (Variables|/Script/Engine.CharacterMovementComponent|SetGroundFriction _charactermovement 8.0)
  (Variables|/Script/Engine.CharacterMovementComponent|SetMaxAcceleration _charactermovement 1.5e+03)
  (Variables|/Script/Engine.CharacterMovementComponent|SetBrakingDecelerationWalking _charactermovement 2e+03)
  (Utilities|Array|RemoveIndex (Variables|Default|GetOverlappin%20Actors) Index))