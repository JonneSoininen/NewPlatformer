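; Gravity platform Blueprint that changes the gravity scale of overlapping characters, building on a parent class for begin play and begin overlap.
; Activate Platform applies the configured GravityScale to an indexed actor's CharacterMovement.
; When a tracked character leaves, the effect lingers for ZeroGravityDuration, then Deactivate Platform restores gravity to 1.0 and removes it from the overlap array.
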(event EventBeginPlay
  (|CallParentFunction))

(event Collision|EventActorBeginOverlap
  (params (OtherActor :type Actor%20Object%20Reference))
  (|CallParentFunction OtherActor))

(event Collision|EventActorEndOverlap
  (params (OtherActor :type Actor%20Object%20Reference))
  (bind _ascharacter (Utilities|Casting|CastToCharacter OtherActor))
  (if (.IsOverlapping1 (CallFunction|CheckOverlapping _ascharacter))
    (Utilities|FlowControl|Delay (Variables|Default|GetZero%20Gravity%20Duration))
    (CallFunction|DeactivatePlatform (.Index (CallFunction|CheckOverlapping _ascharacter)))))

(fn ConstructionScript
  (|CallParentFunction))

(fn ActivatePlatform
  (params (Index :type Integer))
  (Variables|/Script/Engine.CharacterMovementComponent|SetGravityScale (Variables|/Script/Engine.Character|GetCharacterMovement (Utilities|Array|Get(acopy) (Variables|Default|GetOverlappin%20Actors) Index)) (Variables|Default|GetGravity%20Scale)))

(fn DeactivatePlatform
  (params (Index :type Integer))
  (Variables|/Script/Engine.CharacterMovementComponent|SetGravityScale (Variables|/Script/Engine.Character|GetCharacterMovement (Utilities|Array|Get(acopy) (Variables|Default|GetOverlappin%20Actors) Index)) 1.0)
  (Utilities|Array|RemoveIndex (Variables|Default|GetOverlappin%20Actors) Index))