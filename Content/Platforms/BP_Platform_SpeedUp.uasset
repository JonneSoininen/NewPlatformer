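; Speed-boost platform that adds AddSpeed to a character's MaxWalkSpeed and takes it away again after SpeedDuration.
; ActivatePlatform applies the boost but is not called in this graph; overlap tracking uses CheckOverlapArray, which is not defined here.
; End overlap starts a single timer for deactivation.
; DeactivatePlatform restarts it if the character still overlaps the platform, otherwise removes the boost and array entry.
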(event Custom|TriggerDeactivate
  (CallFunction|DeactivatePlatform (.Index (CallFunction|CheckOverlapArray (stale EventActorEndOverlap _ascharacter)))))

(event EventBeginPlay
  (|CallParentFunction) ; This node is disabled and will not be called.\nDrag off pins to build functionality.
)

(event Collision|EventActorBeginOverlap
  (params (OtherActor :type Actor%20Object%20Reference))
  (|CallParentFunction OtherActor) ; This node is disabled and will not be called.\nDrag off pins to build functionality.
)

(event EventActorEndOverlap
  (params (OtherActor :type Actor%20Object%20Reference))
  (bind _ascharacter (Utilities|Casting|CastToCharacter OtherActor))
  (if (.IsOverlapping1 (CallFunction|CheckOverlapArray _ascharacter))
    (bind _returnvalue (Utilities|Time|SetTimerbyEvent (delegate Custom|TriggerDeactivate) (Variables|Default|GetSpeed%20Duration)))
    (Variables|Default|SetTimer _returnvalue)))

(fn ConstructionScript
  (|CallParentFunction))

(fn ActivatePlatform
  (params (Index :type Integer))
  (bind _overlappin_actors (Variables|Default|GetOverlappin%20Actors))
  (bind _output (Utilities|Array|Get(acopy) _overlappin_actors Index))
  (bind _charactermovement (Variables|/Script/Engine.Character|GetCharacterMovement _output))
  (Variables|/Script/Engine.CharacterMovementComponent|SetMaxWalkSpeed _charactermovement (+ (Variables|/Script/Engine.CharacterMovementComponent|GetMaxWalkSpeed _charactermovement) (Variables|Default|GetAdd%20Speed)))
  (Development|PrintString "Activate"))

(fn DeactivatePlatform
  (params (Index :type Integer))
  (bind _overlappin_actors (Variables|Default|GetOverlappin%20Actors))
  (bind _output (Utilities|Array|Get(acopy) _overlappin_actors Index))
  (bind _charactermovement (Variables|/Script/Engine.Character|GetCharacterMovement _output))
  (for _array_element (Collision|GetOverlappingActors (Utilities|Array|Get(acopy) (Variables|Default|GetOverlappin%20Actors) Index) 0 :!class /Script/Engine.Actor)
    (if (== _array_element self)
      (LocalVariables|SetIsOverlapping true)))
  (if (LocalVariables|GetIsOverlapping)
    (Utilities|Time|ClearandInvalidateTimerbyHandle (Variables|Default|GetTimer))
    (bind _returnvalue (Utilities|Time|SetTimerbyEvent (EventDispatchers|CreateEvent :!event Custom|TriggerDeactivate) (Variables|Default|GetSpeed%20Duration)))
    (Variables|Default|SetTimer _returnvalue)
    (else
      (Variables|/Script/Engine.CharacterMovementComponent|SetMaxWalkSpeed _charactermovement (- (Variables|/Script/Engine.CharacterMovementComponent|GetMaxWalkSpeed _charactermovement) (Variables|Default|GetAdd%20Speed)))
      (Development|PrintString "Deactivate")
      (Utilities|Array|RemoveIndex (Variables|Default|GetOverlappin%20Actors) Index))))